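; BP_Tree is a choppable tree that yields wood when the interacting character has an axe.
; Each Interact lowers RemainingAmount, slightly shrinks the mesh, spawns a BP_Wood at the SpawnWood point with an upward impulse and plays a chop sound.
; The tree destroys itself once RemainingAmount runs out.
; GetInteractionName supplies the prompt, showing "Chop" as valid with an axe and "Find an axe" as invalid without one.
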(event `/Game/Blueprints/BI_Interactable.Interact`
  (params (Character :type "/Game/FirstPerson/Blueprints/BP_FirstPersonCharacter Object Reference"))
  (bind _sm_tree_002 (`self.SM_Tree_002`))
  (if (`/Game/FirstPerson/Blueprints/BP_FirstPersonCharacter.hasAxe` Character)
    (bind _output_get (set `self.remainingAmount` (- (`self.remainingAmount`) 0.25)))
    (`SceneComponent.SetRelativeScale3D` _sm_tree_002 (- (`SceneComponent.RelativeScale3D` _sm_tree_002) 0.01))
    (bind _returnvalue (`|SpawnActorFromClass` "/Game/Blueprints/BP_Wood.BP_Wood_C" (`SceneComponent.K2_GetComponentToWorld` (`self.SpawnWood`)) "Undefined" "MultiplyWithRoot" null null))
    (`PrimitiveComponent.AddImpulse` (`/Game/Blueprints/BP_Wood.SM_QuarterCylinder` _returnvalue) (0.0 0.0 10.0) "None" true)
    (`GameplayStatics.PlaySound2D` "/Game/Audio/Sounds/treechop_hollowtonal-100294.treechop_hollowtonal-100294" 1.0 1.0 0.0 null null)
    (if (<= _output_get 0.0)
      (`self.K2_DestroyActor`))))

(fn `GetInteractionName`
  (params (Character :type "/Game/FirstPerson/Blueprints/BP_FirstPersonCharacter Object Reference"))
  (returns (InteractionName :type String) (isValidAction :type Boolean))
  (if (`/Game/FirstPerson/Blueprints/BP_FirstPersonCharacter.hasAxe` Character)
    (return "Chop" true)
    (else
      (return "Find an axe" false))))

(fn `UserConstructionScript`)