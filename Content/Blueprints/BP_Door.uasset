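; Interactable door Blueprint that swings open and closed and supplies an "Open Door" or "Close Door" prompt based on its IsOpen state.
; Interact calls the Toggle dispatcher, which the Blueprint binds to its own event on BeginPlay.
; That event uses a FlipFlop to play or reverse the Door timeline.
; Timeline updates set IsOpen and lerp the Hinge's relative rotation through 90 degrees.
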(event `self.ReceiveBeginPlay`
  (add `self.Toggle` (delegate `Toggle_Event`)))

(event `Toggle_Event`
  (bind _isa (`/Engine/EditorBlueprintResources/StandardMacros.FlipFlop`)
    (:`A`
      (bind (_direction _newtrack_0) (`Timeline|Door` :!label _label)
        (:`Update`
          (set `self.isOpen` _isa)
          (`SceneComponent.K2_SetRelativeRotation` (`self.Hinge`) (`KismetMathLibrary.RLerp` (struct) (struct :`Yaw` 90.0) _newtrack_0) false false))))
    (:`B`
      (goto _label :!via `Reverse`))))

(fn `GetInteractionName`
  (returns (InteractionName :type String))
  (if (`self.isOpen`)
    (return "Close Door")
    (else
      (return "Open Door"))))

(fn `Interact`
  (`self.Toggle`)
  (`KismetSystemLibrary.PrintString` "Calling Toggle")
  (return))

(fn `UserConstructionScript`)