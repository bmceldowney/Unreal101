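; BP_PlaceableObject is a placeable object that shows a valid or invalid spawn preview until it is placed.
; It disables mesh collision on BeginPlay, takes its static mesh through SetMesh, and SwitchMaterial picks the preview material from IsValidSpawn.
; PlaceObject finalizes it by restoring query and physics collision and applying a hard-coded stylized bed material, whatever mesh was set.
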(event `SetMesh`
  (params (Mesh :type "StaticMesh Object Reference"))
  (`StaticMeshComponent.SetStaticMesh` (`self.Mesh`) Mesh))

(event `SwitchMaterial`
  (bind _mesh (`self.Mesh`))
  (if (`self.isValidSpawn`)
    (`PrimitiveComponent.SetMaterial` _mesh 0 "/Game/Materials/M_ValidSpawn.M_ValidSpawn")
    (else
      (`PrimitiveComponent.SetMaterial` _mesh 0 "/Game/Materials/M_InvalidSpawn.M_InvalidSpawn"))))

(event `self.ReceiveBeginPlay`
  (`PrimitiveComponent.SetCollisionEnabled` (`self.Mesh`) "NoCollision"))

(fn `PlaceObject`
  (bind _mesh (`self.Mesh`))
  (`PrimitiveComponent.SetMaterial` _mesh 0 "/Game/Materials/Instances/Stylized/MI_Stylized_Bed.MI_Stylized_Bed")
  (`PrimitiveComponent.SetCollisionEnabled` _mesh "QueryAndPhysics"))

(fn `UserConstructionScript`)